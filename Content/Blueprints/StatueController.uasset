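; AI controller for a Statue pawn that moves only while the player's EyesValue is above a threshold, and otherwise stops with its mesh animation paused.
; Each Tick it branches on the statue's Mode: Bro heads for the player's MarkedLocation, while Bad Dude chases the player and calls DED on UmbraPlayerController upon reaching them.
; Player and statue references are cached at BeginPlay and re-acquired on Tick when invalid.
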(event EventBeginPlay
  (bind _asumbra_character (Utilities|Casting|CastToUmbraCharacter (Game|Player|GetPlayerPawn 0)))
  (Variables|Default|SetPlayer _asumbra_character)
  (bind _asstatue (Utilities|Casting|CastToStatue (Pawn|GetControlledPawn)))
  (Variables|Default|SetStatue _asstatue))

(event EventTick
  (params (DeltaSeconds :type Float%20%28single-precision%29))
  (Utilities|IsValid (Variables|Default|GetPlayer)
    (:Is%20Valid
      (Utilities|IsValid (Variables|Default|GetStatue)
        (:Is%20Valid
          (switch Utilities|FlowControl|Switch|SwitchonStatueAIMode (Variables|/Game/Blueprints/Statue.Statue_C|GetMode (Variables|Default|GetStatue))
            (:NewEnumerator0
              (if (> (Variables|/Script/Umbra.UmbraCharacter|GetEyesValue (Variables|Default|GetPlayer)) 0.75)
                (AI|Navigation|MovetoLocation (Variables|/Script/Umbra.UmbraCharacter|GetMarkedLocation (Variables|Default|GetPlayer)) -1.0 true true false)
                (Variables|/Script/Engine.SkeletalMeshComponent|SetbPauseAnims (Variables|/Script/Engine.Character|GetMesh (Variables|Default|GetStatue)) false :!label _label)
                (else
                  (AI|Navigation|StopMovement)
                  (Variables|/Script/Engine.SkeletalMeshComponent|SetbPauseAnims (Variables|/Script/Engine.Character|GetMesh (Variables|Default|GetStatue)) true :!label _label_2))))
            (:NewEnumerator1
              (if (> (Variables|/Script/Umbra.UmbraCharacter|GetEyesValue (Variables|Default|GetPlayer)) 0.75)
                (bind _returnvalue (AI|Navigation|MovetoActor (Variables|Default|GetPlayer) -1.0 true true))
                (switch Utilities|FlowControl|Switch|SwitchonEPathFollowingRequestResult _returnvalue
                  (:Failed
                    (goto _label))
                  (:AlreadyAtGoal
                    (bind _asumbra_player_controller (Utilities|Casting|CastToUmbraPlayerController (Game|GetPlayerController 0)))
                    (Default|DED _asumbra_player_controller)
                    (goto _label))
                  (:RequestSuccessful
                    (goto _label)))
                (else
                  (AI|Navigation|StopMovement)
                  (goto _label_2))))))
        (:Is%20Not%20Valid
          (bind _asstatue (Utilities|Casting|CastToStatue (Pawn|GetControlledPawn) :!label _label_3))
          (Variables|Default|SetStatue _asstatue))))
    (:Is%20Not%20Valid
      (bind _asumbra_character (Utilities|Casting|CastToUmbraCharacter (Game|Player|GetPlayerPawn 0)))
      (Variables|Default|SetPlayer _asumbra_character)
      (goto _label_3))))

(fn ConstructionScript)