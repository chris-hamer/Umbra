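; Player controller for the Umbra character that creates the HUD and death-screen widgets and runs the death and respawn cycle.
; While the player is alive, Tick writes the character's eye value and the nearest Bad Dude statue's distance to the PlayerInfo parameter collection.
; DED, guarded by a DoOnce, plays the death animation and pauses those updates.
; After a delay, ReAlive teleports player and statues to their home locations.
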(event Custom|ReAlive!
  (Variables|Default|SetState "NewEnumerator0")
  (Rendering|Material|SetScalarParameterValue "/Game/Materials/PlayerInfo.PlayerInfo" "EyeAmount" 0.0 :!class /Script/Engine.KismetMaterialLibrary)
  (Transformation|SetActorLocation (Variables|Default|GetUmbraPlayer) (Variables|Default|GetHome) false true)
  (bind _outactors (Actor|GetAllActorsOfClass "/Game/Blueprints/Statue.Statue_C"))
  (for _array_element _outactors
    (Transformation|SetActorLocation _array_element (Variables|/Game/Blueprints/Statue.Statue_C|GetHome _array_element) false true)
    (Utilities|FlowControl|DoOnce false) ; enters at Reset
  ))

(event Custom|DED
  (Utilities|FlowControl|DoOnce false
    (:Completed
      (Default|PlayAnim (Variables|Default|GetYOUDIED))
      (Variables|Default|SetState "NewEnumerator1")
      (Rendering|Material|SetScalarParameterValue "/Game/Materials/PlayerInfo.PlayerInfo" "EyeAmount" 1.0 :!class /Script/Engine.KismetMaterialLibrary)
      (Utilities|FlowControl|Delay 4.0)
      (CallFunction|ReAlive!))))

(event EventBeginPlay
  (bind _asumbra_character (Utilities|Casting|CastToUmbraCharacter (Pawn|GetControlledPawn)))
  (bind _output_get (Variables|Default|SetUmbraPlayer _asumbra_character))
  (Variables|Default|SetHome (Transformation|GetActorLocation _output_get))
  (Class|PrimitiveComponent|SetPhysMaterialOverride (Variables|/Script/Umbra.UmbraCharacter|GetCapsuleComponent _output_get) "/Game/PlayerPhysMat.PlayerPhysMat")
  (bind _returnvalue (UserInterface|CreateWidget "/Game/Blueprints/HUD.HUD_C" self))
  (bind _output_get_2 (Variables|Default|SetHUD _returnvalue))
  (UserInterface|Viewport|AddtoViewport _output_get_2 0)
  (bind _returnvalue_2 (UserInterface|CreateWidget "/Game/Blueprints/YOUDIED.YOUDIED_C" self))
  (bind _output_get_3 (Variables|Default|SetYOUDIED _returnvalue_2))
  (UserInterface|Viewport|AddtoViewport _output_get_3 0))

(event EventTick
  (params (DeltaSeconds :type Float%20%28single-precision%29))
  (bind _returnvalue (Pawn|GetControlledPawn))
  (if (not (Utilities|Enum|Equal(Enum) (Variables|Default|GetState) "NewEnumerator1"))
    (Utilities|FlowControl|Sequence
      (:then_0
        (bind _asumbra_character (Utilities|Casting|CastToUmbraCharacter _returnvalue)))
      (:then_1
        (Utilities|IsValid (Variables|Default|GetUmbraPlayer)
          (:Is%20Valid
            (Rendering|Material|SetScalarParameterValue "/Game/Materials/PlayerInfo.PlayerInfo" "EyeAmount" (Variables|/Script/Umbra.UmbraCharacter|GetEyesValue (Variables|Default|GetUmbraPlayer)) :!class /Script/Engine.KismetMaterialLibrary))
          (:Is%20Not%20Valid
            (bind _asumbra_character_2 (Utilities|Casting|CastToUmbraCharacter _returnvalue))
            (bind _output_get (Variables|Default|SetUmbraPlayer _asumbra_character_2))
            (Variables|Default|SetHome (Transformation|GetActorLocation _output_get))
            (Class|PrimitiveComponent|SetPhysMaterialOverride (Variables|/Script/Umbra.UmbraCharacter|GetCapsuleComponent _output_get) "/Game/PlayerPhysMat.PlayerPhysMat")
            (bind _returnvalue_2 (UserInterface|CreateWidget "/Game/Blueprints/HUD.HUD_C" self))
            (bind _output_get_2 (Variables|Default|SetHUD _returnvalue_2))
            (UserInterface|Viewport|AddtoViewport _output_get_2 0)
            (bind _returnvalue_3 (UserInterface|CreateWidget "/Game/Blueprints/YOUDIED.YOUDIED_C" self))
            (bind _output_get_3 (Variables|Default|SetYOUDIED _returnvalue_3))
            (UserInterface|Viewport|AddtoViewport _output_get_3 0))))
      (:then_2
        (bind _outactors (Actor|GetAllActorsOfClass "/Game/Blueprints/Statue.Statue_C"))
        (Rendering|Material|SetScalarParameterValue "/Game/Materials/PlayerInfo.PlayerInfo" "DistanceToClosestBadDude" 1e+03 :!class /Script/Engine.KismetMaterialLibrary)
        (for _array_element _outactors
          (switch Utilities|FlowControl|Switch|SwitchonStatueAIMode (Variables|/Game/Blueprints/Statue.Statue_C|GetMode _array_element)
            (:NewEnumerator1
              (bind _returnvalue_4 (Rendering|Material|GetScalarParameterValue "/Game/Materials/PlayerInfo.PlayerInfo" "DistanceToClosestBadDude" :!class /Script/Engine.KismetMaterialLibrary))
              (if (> _returnvalue_4 (Transformation|GetDistanceTo _array_element (Variables|Default|GetUmbraPlayer)))
                (Rendering|Material|SetScalarParameterValue "/Game/Materials/PlayerInfo.PlayerInfo" "DistanceToClosestBadDude" (Transformation|GetDistanceTo _array_element (Variables|Default|GetUmbraPlayer)) :!class /Script/Engine.KismetMaterialLibrary)))))))))

(fn ConstructionScript)