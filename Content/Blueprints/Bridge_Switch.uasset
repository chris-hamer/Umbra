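; Pressure-switch actor that shows or hides a linked Bridge while the UmbraCharacter or a Statue overlaps it.
; Overlap begin and end events adjust an occupant counter, with the Permanent flag skipping decrements so the switch stays on.
; Every Tick, unless the No flag is set, the counter drives the Bridge mesh's visibility and collision.
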(event EventBeginPlay)

(event Collision|EventActorBeginOverlap
  (params (OtherActor :type Actor%20Object%20Reference))
  (Utilities|Casting|CastToUmbraCharacter OtherActor
    (:then
      _)
    (:CastFailed
      (Utilities|Casting|CastToStatue OtherActor)))
  (Math|Integer|IncrementInt (Variables|Default|GetN)))

(event Collision|EventActorEndOverlap
  (params (OtherActor :type Actor%20Object%20Reference))
  (if (not (Variables|Default|Getpermanent))
    (Utilities|Casting|CastToUmbraCharacter OtherActor
      (:then
        _)
      (:CastFailed
        (Utilities|Casting|CastToStatue OtherActor)))
    (Math|Integer|DecrementInt (Variables|Default|GetN))))

(event EventTick
  (params (DeltaSeconds :type Float%20%28single-precision%29))
  (bind _bridge (Variables|Default|GetBridge))
  (bind _n (Variables|Default|GetN))
  (bind _returnvalue (>= _n 1))
  (bind _staticmesh (Variables|/Game/Blueprints/Bridge.Bridge_C|GetStaticMesh _bridge))
  (if (not (Variables|Default|Getno))
    (Rendering|SetVisibility _staticmesh _returnvalue false)
    (Collision|SetCollisionEnabled _staticmesh (select _returnvalue "QueryAndPhysics" "NoCollision"))))

(fn ConstructionScript)